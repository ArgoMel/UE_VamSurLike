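; BP_PhotoBooth is a capture actor that renders skeletal mesh portraits and saves them as static textures through an editor-only call.
; GeneratePortrait rotates the spring arm, assigns the mesh and sizes the orthographic scene capture from its bounds radius; bounds-based camera repositioning is left unconnected.
; TakePicture runs this on the current mesh, then saves RT_Portrait as a T_-prefixed texture, with a stray submix SetDelayLength call in between.
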(event Custom|GeneratePortrait
  (params (SM :type Skeletal%20Mesh%20Object%20Reference) (Rotation :type Rotator))
  (Transformation|AddRelativeRotation (Variables|Default|GetSpringArm) Rotation false false)
  (Components|SkeletalMesh|SetSkeletalMeshAsset (Variables|Default|GetSkeletalMesh) SM)
  (Variables|/Script/Engine.SceneCaptureComponent2D|SetOrthoWidth (Variables|Default|GetSceneCaptureComponent2D) (* (.sphereradius (StaticMesh|GetBounds SM)) 2.1))
  (Rendering|SceneCapture|ShowOnlyComponent (Variables|Default|GetSceneCaptureComponent2D) 0))

(event EventBeginPlay)

(event Collision|EventActorBeginOverlap
  (params (OtherActor :type Actor%20Object%20Reference)))

(event EventTick
  (params (DeltaSeconds :type Float%20%28single-precision%29)))

(fn ConstructionScript)

(fn TakePicture
  (bind _skeletalmesh (Variables|Default|GetSkeletalMesh))
  (bind _returnvalue (Components|SkeletalMesh|GetSkeletalMeshAsset _skeletalmesh))
  (CallFunction|GeneratePortrait _returnvalue "0, 0, 0")
  (Class|SubmixEffectDelayStatics|SetDelayLength (Utilities|Struct|MakeSubmixEffectDelaySettings 2e+03 4e+02 1.0) 1.0)
  (Class|KismetRenderingLibrary|RenderTargetCreateStaticTexture2DEditorOnly "/Game/0_KBJ/Texture/Portrait/RT_Portrait.RT_Portrait" (Utilities|String|ToString(Text) (Utilities|Text|MakeLiteralText (Utilities|Text|FormatText "T_{name}" (Utilities|GetDisplayName _returnvalue)))) "TC_Default" "TMGS_Blur1"))