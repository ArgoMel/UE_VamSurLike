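; BP_Checkpoint is a checkpoint actor showing an icon with the player's distance in meters, plus its own minimap icon.
; On BeginPlay it sets up both widgets and attaches a CalcHelper component to the player's root.
; Each tick moves CalcHelper to the checkpoint, using its relative location as the player-relative minimap position, and refreshes the distance text.
; GetMapIconData exposes its location, icon, size and actor reference.
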(event EventBeginPlay
  (bind _aswbp_check_point (Utilities|Casting|CastToWBP_CheckPoint (UserInterface|GetWidget (Variables|Default|GetWidget%20checkpoint))))
  (bind _output_get (Variables|Default|SetCheckpoint _aswbp_check_point))
  (Default|UpdateIcon _output_get (Variables|Default|Geticon) "(X=40.000000,Y=40.000000)")
  (Utilities|FlowControl|Delay 0.2)
  (bind _returnvalue (UserInterface|CreateWidget "/Game/0_KBJ/Minimap/UI/WBP_MinimapIcon.WBP_MinimapIcon_C"))
  (bind _output_get_2 (Variables|Default|SetMinimapIcon _returnvalue))
  (Default|ChangeIcon _output_get_2 (Variables|Default|Geticon))
  (Default|ChangeSize _output_get_2 (Variables|Default|Geticon%20size))
  (UserInterface|Viewport|AddtoViewport _output_get_2 0)
  (Transformation|AttachComponentToComponent (Variables|Default|Getcalc_helper) (Variables|/Script/Engine.Actor|GetRootComponent (Game|GetPlayerCharacter 0)) "None" "KeepWorld" "KeepWorld" "KeepWorld" true)
  (CallFunction|UpdateIconPosition))

(event Collision|EventActorBeginOverlap
  (params (OtherActor :type Actor%20Object%20Reference)))

(event EventTick
  (params (DeltaSeconds :type Float%20%28single-precision%29))
  (CallFunction|UpdateIconPosition)
  (Default|SetText (Variables|Default|GetCheckpoint) (Utilities|Text|ToText(String) (Utilities|String|Append (Utilities|String|ToString(Integer) (Math|Float|Truncate (/ (Math|Vector|Distance(Vector) (Transformation|GetActorLocation (Game|GetPlayerCharacter 0)) (Transformation|GetActorLocation)) 1e+02))) " m"))))

(fn ConstructionScript
  (bind _aswbp_check_point (Utilities|Casting|CastToWBP_CheckPoint (UserInterface|GetWidget (Variables|Default|GetWidget%20checkpoint)))
    (:then
      (Default|UpdateIcon _aswbp_check_point (Variables|Default|Geticon) "(X=40.000000,Y=40.000000)"))
    (:CastFailed
      (Development|PrintString "checkpoint cast fail"))))

(fn UpdateIconPosition
  (bind _minimapicon (Variables|Default|GetMinimapIcon))
  (Transformation|SetWorldLocation (Variables|Default|Getcalc_helper) (Transformation|GetActorLocation) false false)
  (Utilities|IsValid _minimapicon
    (:Is%20Valid
      (Default|UpdateIconLocation _minimapicon (Math|Conversions|ToVector2D(Vector) (Variables|/Script/Engine.SceneComponent|GetRelativeLocation (Variables|Default|Getcalc_helper))) 0.0))))

(fn GetMapIconData
  (return (Transformation|GetActorLocation) (Variables|Default|Geticon) (Variables|Default|Geticon%20size) (Math|Float|MakeLiteralFloat 0.0) self))