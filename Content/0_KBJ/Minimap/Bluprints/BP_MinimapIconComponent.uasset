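; Actor component that shows its owner on the minimap through its own WBP_MinimapIcon widget, created shortly after BeginPlay with the configured icon and size.
; A helper scene component attached to the player character's root is moved to the owner's world transform each tick.
; Its resulting relative location and yaw give the player-relative position and angle for the widget, avoiding manual transform math.
; GetMapIconData exposes location, icon and size.
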(event EventBeginPlay
  (Utilities|FlowControl|Delay 0.2)
  (bind _returnvalue (UserInterface|CreateWidget "/Game/0_KBJ/Minimap/UI/WBP_MinimapIcon.WBP_MinimapIcon_C"))
  (bind _output_get (Variables|Default|SetMinimapIcon _returnvalue))
  (Default|ChangeIcon _output_get (Variables|Default|Geticon))
  (Default|ChangeSize _output_get (Variables|Default|GetIconSize))
  (UserInterface|Viewport|AddtoViewport _output_get 0)
  (bind _returnvalue_2 (Game|AddComponentbyClass (Components|GetOwner) "/Script/Engine.SceneComponent" false))
  (Variables|Default|SetCalcHelper _returnvalue_2)
  (Transformation|AttachComponentToComponent (Variables|Default|GetCalcHelper) (Variables|/Script/Engine.Actor|GetRootComponent (Game|GetPlayerCharacter 0)) "None" "KeepWorld" "KeepWorld" "KeepWorld" true))

(event EventTick
  (params (DeltaSeconds :type Float%20%28single-precision%29))
  (CallFunction|UpdateIconPosition))

(fn UpdateIconPosition
  (bind _returnvalue (Components|GetOwner))
  (bind _minimapicon (Variables|Default|GetMinimapIcon))
  (bind _calchelper (Variables|Default|GetCalcHelper))
  (bind _calchelper_2 (Variables|Default|GetCalcHelper))
  (Utilities|IsValid _calchelper_2
    (:Is%20Valid
      (Transformation|SetWorldLocationAndRotation _calchelper_2 (Transformation|GetActorLocation _returnvalue) (Transformation|GetActorRotation _returnvalue) false false)
      (Utilities|IsValid _minimapicon
        (:Is%20Valid
          (Default|UpdateIconLocation _minimapicon (Math|Conversions|ToVector2D(Vector) (Variables|/Script/Engine.SceneComponent|GetRelativeLocation _calchelper)) (.yaw (Variables|/Script/Engine.SceneComponent|GetRelativeRotation _calchelper))))))))

(fn GetMapIconData
  (return (Transformation|GetActorLocation (Components|GetOwner)) (Variables|Default|Geticon) (Variables|Default|GetIconSize)))