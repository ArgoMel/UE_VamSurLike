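; Prototype character Blueprint for testing weapon fire and mouse-to-world positioning.
; BeginPlay loops a one-second timer into TestShooting, which spawns at the LLWeapon muzzle socket with the actor's rotation, though its spawn node shows no class.
; Keys 1 and 2 compare cursor deprojection with a Visibility hit trace, printing each position and placing a temporary TestSphere.
; Unwired line-trace and MyProtoProjectile spawn experiments remain in the event graph.
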(event EventBeginPlay
  (Utilities|Time|SetTimerbyFunctionName 0 "TestShooting" 1.0 true))

(event Collision|EventActorBeginOverlap
  (params (OtherActor :type Actor%20Object%20Reference)))

(event EventTick
  (params (DeltaSeconds :type Float%20%28single-precision%29)))

(event Input|KeyboardEvents|1
  (params (Key :type Key%20Structure :default "None"))
  (:Pressed
    (bind _asproto_player_controller (Utilities|Casting|CastToProtoPlayerController (Game|GetPlayerController 0)))
    (if (.ReturnValue (Game|Player|ConvertMouseLocationToWorldSpace _asproto_player_controller))
      (Development|PrintString (Utilities|String|Append "Convert Mouse 
" (Utilities|String|ToString(Vector) (.WorldLocation (Game|Player|ConvertMouseLocationToWorldSpace _asproto_player_controller)))) true true "(R=0.014199,G=1.000000,B=0.000000,A=1.000000)" 1e+01)
      (bind _returnvalue (Game|SpawnActorfromClass "/Game/2_HHS/Blueprint/TestSphere.TestSphere_C" (Math|Transform|MakeTransform (.WorldLocation (Game|Player|ConvertMouseLocationToWorldSpace _asproto_player_controller)) "0, 0, 0" "1.000000,1.000000,1.000000") "Undefined" "MultiplyWithRoot" 0 0))
      (Utilities|FlowControl|Delay 1e+01)
      (Actor|DestroyActor _returnvalue)
      (else
        (Development|PrintString "계산 실패" true true "(R=1.000000,G=0.029464,B=0.000000,A=1.000000)")))))

(event Input|KeyboardEvents|2
  (params (Key :type Key%20Structure :default "None"))
  (:Pressed
    (bind _asproto_player_controller (Utilities|Casting|CastToProtoPlayerController (Game|GetPlayerController 0)))
    (if (.ReturnValue (Game|Player|GetHitResultUnderCursorbyChannel _asproto_player_controller "TraceTypeQuery1" true))
      (Development|PrintString (Utilities|String|Append "Under Cursor 
" (Utilities|String|ToString(Vector) (.Location (Collision|BreakHitResult (.HitResult (Game|Player|GetHitResultUnderCursorbyChannel _asproto_player_controller "TraceTypeQuery1" true)))))) true true "(R=1.000000,G=0.819961,B=0.000000,A=1.000000)" 1e+01)
      (bind _returnvalue (Game|SpawnActorfromClass "/Game/2_HHS/Blueprint/TestSphere.TestSphere_C" (Math|Transform|MakeTransform (.Location (Collision|BreakHitResult (.HitResult (Game|Player|GetHitResultUnderCursorbyChannel _asproto_player_controller "TraceTypeQuery1" true)))) "0, 0, 0" "1.000000,1.000000,1.000000") "Undefined" "MultiplyWithRoot" 0 0))
      (Utilities|FlowControl|Delay 1e+01)
      (Actor|DestroyActor _returnvalue)
      (else
        (Development|PrintString "계산 실패" true true "(R=1.000000,G=0.029464,B=0.000000,A=1.000000)")))))

(fn ConstructionScript)

(fn TestShooting
  (Game|SpawnActorfromClass "/Game/2_HHS/Blueprint/MyProtoProjectile.MyProtoProjectile_C" (Math|Transform|MakeTransform (Transformation|GetSocketLocation (Variables|Default|GetLLWeapon) "b_gun_muzzleflash") (Transformation|GetActorRotation) "1.000000,1.000000,1.000000") "AlwaysSpawn" "MultiplyWithRoot" 0 0))