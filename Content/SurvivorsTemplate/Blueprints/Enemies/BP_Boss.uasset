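; BP_Boss is a boss enemy Blueprint for the Survivors template that varies its attack animation.
; Its MCEnemyAttack event rolls a random integer and plays one of ten Crunch montages at normal rate.
; The random pick happens inside the event itself, so each execution rolls independently.
; It adds no other behavior: BeginPlay, overlap and Tick are inactive stubs, and the construction script only calls its parent.
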(event EventBeginPlay
  (|CallParentFunction) ; 지금 이 노드는 비활성 상태입니다. \n핀을 끌어서 다른 노드를 연결하면 활성화됩니다.
)

(event Collision|EventActorBeginOverlap
  (params (OtherActor :type Actor%20Object%20Reference)))

(event EventTick
  (params (DeltaSeconds :type Float%20%28single-precision%29)))

(event EventMCEnemyAttack
  (switch int (Math|Random|RandomInteger 10)
    (:0
      (Animation|PlayAnimMontage "/Game/AI/Animation/AM_Crunch.AM_Crunch" 1.0 "None"))
    (:1
      (Animation|PlayAnimMontage "/Game/AI/Animation/AM_2Crunch.AM_2Crunch" 1.0 "None"))
    (:2
      (Animation|PlayAnimMontage "/Game/AI/Animation/AM_3Crunch.AM_3Crunch" 1.0 "None"))
    (:3
      (Animation|PlayAnimMontage "/Game/AI/Animation/AM_4Crunch.AM_4Crunch" 1.0 "None"))
    (:4
      (Animation|PlayAnimMontage "/Game/AI/Animation/AM_5Crunch.AM_5Crunch" 1.0 "None"))
    (:5
      (Animation|PlayAnimMontage "/Game/AI/Animation/AM_6Crunch.AM_6Crunch" 1.0 "None"))
    (:6
      (Animation|PlayAnimMontage "/Game/AI/Animation/AM_7Crunch.AM_7Crunch" 1.0 "None"))
    (:7
      (Animation|PlayAnimMontage "/Game/AI/Animation/AM_8Crunch.AM_8Crunch" 1.0 "None"))
    (:8
      (Animation|PlayAnimMontage "/Game/AI/Animation/AM_9Crunch.AM_9Crunch" 1.0 "None"))
    (:9
      (Animation|PlayAnimMontage "/Game/AI/Animation/AM_10Crunch.AM_10Crunch" 1.0 "None"))))

(fn ConstructionScript
  (|CallParentFunction))