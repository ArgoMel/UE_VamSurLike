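; Base game instance for the Survivors template, handling default character selection, lobby character spawning and session failures.
; On Init it stores the first row of DT_AvailableCharacters as the Player data.
; Network and travel errors print the failure type and destroy the session.
; SpawnCharacter replaces the previous lobby character with a synchronously loaded, non-replicated BP_Lobby_Character at the transform of the first Pawn found.
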(event EventHandleNetworkError
  (params (FailureType :type ENetworkFailure%20Enum :default "NetDriverAlreadyExists") (bIsServer :type Boolean))
  (Development|PrintString (Utilities|String|EnumtoString FailureType) true true "(R=1.000000,G=0.000000,B=0.000000,A=1.000000)" 1e+01)
  (|DestroySession (Game|GetPlayerController 0)))

(event EventHandleTravelError
  (params (FailureType :type ETravelFailure%20Enum :default "NoLevel"))
  (Development|PrintString (Utilities|String|EnumtoString FailureType) true true "(R=1.000000,G=0.000000,B=0.000000,A=1.000000)" 1e+01)
  (|DestroySession (Game|GetPlayerController 0)))

(event EventInit
  (bind _outrownames (DataTable|GetDataTableRowNames "/Game/SurvivorsTemplate/Blueprints/DataTables/DT_AvailableCharacters.DT_AvailableCharacters"))
  (bind _returnvalue (Utilities|GetDataTableRow "/Game/SurvivorsTemplate/Blueprints/DataTables/DT_AvailableCharacters.DT_AvailableCharacters" (Utilities|Array|Get(acopy) _outrownames))
    (:then
      (Variables|Default|SetPlayer _returnvalue))))

(fn SpawnCharacter
  (bind _lastplayerclass (Variables|Default|GetLastPlayerClass)
    (:then
      (Actor|DestroyActor _lastplayerclass))
    (:else
      _))
  (bind _returnvalue (Utilities|LoadClassAssetBlocking "/Game/SurvivorsTemplate/Blueprints/Character/BP_Lobby_Character.BP_Lobby_Character_C"))
  (bind _as액터 (Utilities|Casting|CastToActorClass _returnvalue))
  (bind _returnvalue_2 (Actor|GetActorOfClass "/Script/Engine.Pawn"))
  (bind _returnvalue_3 (Game|SpawnActorfromClass _as액터 (Transformation|GetActorTransform _returnvalue_2) "Undefined" "SelectDefaultAtRuntime" 0 0))
  (Variables|Default|SetLastPlayerClass _returnvalue_3)
  (Networking|SetReplicates _returnvalue_3 false))