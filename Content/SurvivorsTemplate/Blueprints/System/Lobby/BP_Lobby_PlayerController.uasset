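; Lobby player controller that sets up the lobby menu and character for the local player.
; On BeginPlay it clears widgets, shows WB_LobbyMenu with game-and-UI input, and has the game instance spawn a character.
; It then passes the game instance's LastPlayerClass to ChangePlayer, which possesses it if it casts to BP_Lobby_Character.
; Player joins trigger an update of the menu's player total from the GameState's PlayerArray.
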(event Custom|OC_UpdatePlayerTotal
  ;[1 1 1] Update Player Count
  (Default|UpdatePlayerTotal (Variables|Default|GetPlayerHud) (Utilities|Array|Length (Variables|/Script/Engine.GameStateBase|GetPlayerArray (Game|GetGameState)))))

(event EventBeginPlay
  ;[1 1 1] Prepare UI
  (if (Pawn|IsLocalPlayerController)
    (Viewport|RemoveAllWidgets)
    (CallFunction|CreateUI)
    (bind _asbp_base_game_instance (Utilities|Casting|CastToBP_Base_GameInstance (Game|GetGameInstance)))
    (Default|SpawnCharacter _asbp_base_game_instance)
    (CallFunction|ChangePlayer (Variables|/Game/SurvivorsTemplate/Blueprints/System/BP_Base_GameInstance.BP_Base_GameInstance_C|GetLastPlayerClass _asbp_base_game_instance))))

(event EventOnPlayerJoin
  ;[1 1 1] Update Player Count
  (CallFunction|OCUpdatePlayerTotal))

(fn ConstructionScript)

(fn CreateUI
  (bind _playerhud (Variables|Default|GetPlayerHud)
    (:then
      (if (not (UserInterface|Viewport|IsinViewport _playerhud))
        (UserInterface|Viewport|AddtoViewport (stale _output_get) 0 :!label _label)
        (Input|SetInputModeGameandUI self (Variables|Default|GetPlayerHud) "DoNotLock" false false)))
    (:else
      (bind _returnvalue (UserInterface|CreateWidget "/Game/SurvivorsTemplate/Widgets/WB_LobbyMenu.WB_LobbyMenu_C" self))
      (bind _output_get (Variables|Default|SetPlayerHud _returnvalue))
      (goto _label))))

(fn ChangePlayer
  (params (Object :type Object%20Object%20Reference))
  (bind _asbp_lobby_character (Utilities|Casting|CastToBP_Lobby_Character Object))
  (Pawn|Possess _asbp_lobby_character))